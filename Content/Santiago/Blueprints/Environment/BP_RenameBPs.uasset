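; BP_RenameBPs is a utility Blueprint that batch-renames the editor labels of actors of a chosen class.
; When the BPs condition passes, its Rename event gathers all actors of ActorClassRef.
; It labels each with ActorName plus its array index, marking it dirty and printing the new name on screen.
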(event Custom|Rename
  (if (Variables|Default|GetBPs)
    (bind _outactors (Actor|GetAllActorsOfClass 0 (Variables|Default|GetActorClassRef)))
    (for (_array_element _array_index) _outactors
      (EditorScripting|ActorEditing|SetActorLabel _array_element (Utilities|String|Append (Variables|Default|GetActorName) (Utilities|String|ToString(Integer) _array_index)) true)
      (Development|PrintString 0 (Utilities|String|Append (Variables|Default|GetActorName) (Utilities|String|ToString(Integer) _array_index)) true true "(R=0.000000,G=0.649305,B=0.025763,A=1.000000)" 5.0))
    (Utilities|Array|Clear (Utilities|Array|MakeArray _array_index))))

(fn ConstructionScript)